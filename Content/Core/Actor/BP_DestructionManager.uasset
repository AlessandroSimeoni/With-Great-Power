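; BP_DestructionManager is an actor that tracks the combined destruction level of registered destructible elements.
; AddDestructible adds each item's level to a running total and binds to its destroyed event.
; After a short BeginPlay delay, the accumulated total becomes the maximum and a value-changed notification fires.
; Each destroyed BP_DestructibleElement is removed from the item list and subtracted from the total, firing that notification again.
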(event `self.ReceiveBeginPlay`
  (`KismetSystemLibrary.Delay` 0.2)
  (set `self.MaxDestruction_Level` (`self.ActualDestruction Level`))
  (`self.DestructionValueChanged`))

(event `AddDestructible`
  (params (Item :type "/Game/Core/Actor/BP_DestructibleElement Object Reference"))
  (add `Destructible.OnDestroyedCollection` Item (delegate `EventDestroyed`))
  (set `self.ActualDestruction Level` (+ (`Destructible.DestructionLevel` Item) (`self.ActualDestruction Level`))))

(event `EventDestroyed`
  (params (actor :type "Actor Object Reference") (DestructionLevel :type Integer))
  (bind _asbp_destructible_element (cast `/Game/Core/Actor/BP_DestructibleElement` actor))
  (`KismetArrayLibrary.Array_RemoveItem` (`self.DestructableItems`) _asbp_destructible_element)
  (set `self.ActualDestruction Level` (- (`self.ActualDestruction Level`) DestructionLevel))
  (`self.DestructionValueChanged`))

(fn `UserConstructionScript`)