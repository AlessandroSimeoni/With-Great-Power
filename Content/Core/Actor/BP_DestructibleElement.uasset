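; A destructible Chaos geometry collection actor that shatters when overlapped and spawns enemies afterwards.
; Any overlap before breaking briefly spawns a BP_MasterField angled from the other actor's position toward the element.
; The first Chaos break event disables navigation influence collision, reveals a static mesh, calls TriggerDestruction, and plays Niagara, camera shake and sound.
; Timers then hide the debris with physics off and call SpawnEnemies at the spawn point.
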(event `OnActorBeginOverlap_Event` :!signature `self.OnActorBeginOverlap`
  (params (OverlappedActor :type "Actor Object Reference") (OtherActor :type "Actor Object Reference"))
  (bind _returnvalue (`self.K2_GetActorLocation`))
  (bind (_returnvalue_roll _returnvalue_pitch _returnvalue_yaw) (`KismetMathLibrary.BreakRotator` (`KismetMathLibrary.MakeRotFromZ` (- _returnvalue (`self.K2_GetActorLocation` OtherActor)))))
  (if (not (`self.bBroken`))
    (bind _returnvalue_2 (`|SpawnActorFromClass` "/Game/Core/Actor/BP_MasterField.BP_MasterField_C" (`KismetMathLibrary.MakeTransform` (`self.K2_GetActorLocation` OtherActor) (`KismetMathLibrary.MakeRotator` (+ _returnvalue_roll 40.0) _returnvalue_pitch _returnvalue_yaw)) "AlwaysSpawn" "MultiplyWithRoot" null null))
    (`SceneComponent.K2_SetWorldLocation` (`self.Niagara`) _returnvalue false false)
    (`KismetSystemLibrary.Delay` 0.2)
    (`self.K2_DestroyActor` _returnvalue_2)))

(event `self.ReceiveBeginPlay`
  (add `GeometryCollectionComponent.OnChaosBreakEvent` (`self.GeometryCollection`) (delegate `OnChaosBreakEvent_Event`))
  (add `self.OnActorBeginOverlap` (delegate `OnActorBeginOverlap_Event`)))

(event `OnChaosBreakEvent_Event`
  (params (BreakEvent :type "ChaosBreakEvent Structure (by ref)"))
  (if (not (`self.bBroken`))
    (`PrimitiveComponent.SetCollisionEnabled` (`self.NavigationInfluence`) "NoCollision")
    (`SceneComponent.SetVisibility` (`self.StaticMesh`) true true)
    (set `self.bBroken` true)
    (`KismetSystemLibrary.K2_SetTimerDelegate` (delegate `EndDestruction`) (`self.DestroyTimeAfterBreak`))
    (`self.TriggerDestruction`)
    (`ActorComponent.Activate` (`self.Niagara1`) true)
    (`GameplayStatics.PlayWorldCameraShake` "/Game/Camera/BP_CameraShake.BP_CameraShake_C" (`self.K2_GetActorLocation` (`GameplayStatics.GetPlayerPawn` 0)) 0.0 5000.0)
    (`KismetSystemLibrary.K2_SetTimerDelegate` (delegate `Spawn`) (`self.TimeToSpawnAfterDestruction`))
    (`GameplayStatics.PlaySoundAtLocation` (`self.Sound`) (`self.K2_GetActorLocation`) (struct) 1.0 1.0 0.0 "/Game/Audio/SA_base.SA_base" null null null)))

(event `EndDestruction`
  (`self.Destroy`))

(event `Spawn`
  (`self.SpawnEnemies` (`SceneComponent.K2_GetComponentLocation` (`self.SpawnPoint`))))

(fn `Destroy`
  (bind _geometrycollection (`self.GeometryCollection`))
  (`PrimitiveComponent.SetSimulatePhysics` _geometrycollection false)
  (`SceneComponent.SetVisibility` _geometrycollection false true))

(fn `UserConstructionScript`)