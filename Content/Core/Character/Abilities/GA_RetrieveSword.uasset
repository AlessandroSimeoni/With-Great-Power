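; Gameplay ability that returns the main character's thrown sword.
; On activation it calls RetrieveSword on the avatar and waits for the SwordRetrieved gameplay event.
; When the event arrives it switches the player controller's cursor widget to the sword sprite and ends.
; On ability end it removes the loose SwordThrew tag from the avatar without replication.
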(event `self.K2_ActivateAbility`
  (bind _asbp_main_character (cast `/Game/Core/Character/BP_MainCharacter` (`self.GetAvatarActorFromActorInfo`)))
  (`/Game/Core/Character/BP_MainCharacter.RetrieveSword` _asbp_main_character)
  (`AbilityTask_WaitGameplayEvent.WaitGameplayEvent` (struct :`TagName` "Event.SwordRetrieved") null
    (:`EventReceived`
      (`/Game/UI/W_Cursor.ChangeSprite` (`/Game/Core/Character/BP_CharacterController.CursorWIdget` (cast `/Game/Core/Character/BP_CharacterController` (`GameplayStatics.GetPlayerController` 0) :!pure true)) true false)
      (`self.K2_EndAbility`))))

(event `self.K2_OnEndAbility`
  (params (bWasCancelled :type Boolean))
  (`AbilitySystemBlueprintLibrary.RemoveLooseGameplayTags` (`self.GetAvatarActorFromActorInfo`) (`self.SwordThrewTag`)))