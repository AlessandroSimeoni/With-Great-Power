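; Gameplay ability that applies incoming damage to a character and triggers death when health runs out.
; Activated by a gameplay event, it negates the event magnitude, passes it as a SetByCaller value to GE_UpdateHealth on the owner, then ends.
; On end, it reads Health from PlayerAttributeSet and, at zero or below, activates abilities matching DeathTag on the avatar's ability system component.
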(event `self.K2_ActivateAbilityFromEvent`
  (params (EventData :type "GameplayEventData Structure (by ref)"))
  (bind _returnvalue (`AbilitySystemBlueprintLibrary.AssignTagSetByCallerMagnitude` (`self.MakeOutgoingGameplayEffectSpec` "/Game/Core/Character/Effects/GE_UpdateHealth.GE_UpdateHealth_C") (struct :`TagName` "Data.Character.HealthValueModifier") (* EventData_EventMagnitude -1.0)))
  (`self.K2_ApplyGameplayEffectSpecToOwner` _returnvalue)
  (`self.K2_EndAbility`))

(event `self.K2_OnEndAbility`
  (params (bWasCancelled :type Boolean))
  (bind _returnvalue (`AbilitySystemComponent.GetAttributeSet` (`self.GetAbilitySystemComponentFromActorInfo`) "/Script/KenneyJam.PlayerAttributeSet"))
  (bind _asplayer_attribute_set (cast `PlayerAttributeSet` _returnvalue))
  (if (<= (`.CurrentValue` (break `GameplayAttributeData` (`PlayerAttributeSet.Health` _asplayer_attribute_set))) 0.0)
    (`AbilitySystemComponent.TryActivateAbilitiesByTag` (`AbilitySystemBlueprintLibrary.GetAbilitySystemComponent` (`self.GetAvatarActorFromActorInfo`)) (`self.DeathTag`) true)))