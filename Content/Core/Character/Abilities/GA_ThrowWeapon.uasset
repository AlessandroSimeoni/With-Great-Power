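; Gameplay ability that releases the main character's charged sword throw.
; On activation it clears the begin-throw tag, plays the throw montage from its EndLoop section and stops the charge bar.
; A Event.ThrowSword gameplay event triggers the throw, applies a SetByCaller speed effect, switches the cursor from sword to hand and ends the ability.
; OnEndAbility always adds the sword-thrown tag as a non-replicated loose tag.
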(event `self.K2_ActivateAbility`
  (bind _returnvalue (`self.GetAvatarActorFromActorInfo`))
  (`AbilitySystemBlueprintLibrary.RemoveLooseGameplayTags` _returnvalue (`self.BeginThrowTag`))
  (`AbilityTask_PlayMontageAndWait.CreatePlayMontageAndWaitProxy` "None" "/Game/AssetPack/CharacterPack/AnimationsSequence/AM_WeaponThrowSeparete.AM_WeaponThrowSeparete" 1.0 "EndLoop"
    (:`then`
      (bind _asbp_main_character (cast `/Game/Core/Character/BP_MainCharacter` _returnvalue))
      (`/Game/Core/Character/BP_MainCharacter.StopChargeBar` _asbp_main_character)
      (`AbilityTask_WaitGameplayEvent.WaitGameplayEvent` (struct :`TagName` "Event.ThrowSword") null
        (:`EventReceived`
          (`/Game/Core/Character/BP_MainCharacter.ThrowSword` _asbp_main_character)
          (`KismetSystemLibrary.PrintText` (`|FormatText` "THROW, Strength: {perc}" (`ProgressBar.Percent` (`/Game/UI/W_AttackProgress.ProgressBar_0` (`/Game/Core/Character/BP_MainCharacter.AttackProgressBarWidget` _asbp_main_character)))))
          (bind _returnvalue_2 (`AbilitySystemBlueprintLibrary.AssignTagSetByCallerMagnitude` (`self.MakeOutgoingGameplayEffectSpec` "/Game/Core/Character/Effects/GE_UpdatePlayerSpeed.GE_UpdatePlayerSpeed_C") (struct :`TagName` "Data.Character.PlayerSpeedModifier") 1000.0))
          (`self.K2_ApplyGameplayEffectSpecToOwner` _returnvalue_2)
          (`/Game/UI/W_Cursor.ChangeSprite` (`/Game/Core/Character/BP_CharacterController.CursorWIdget` (cast `/Game/Core/Character/BP_CharacterController` (`GameplayStatics.GetPlayerController` 0) :!pure true)) false true)
          (`self.K2_EndAbility`))))))

(event `self.K2_OnEndAbility`
  (params (bWasCancelled :type Boolean))
  (`AbilitySystemBlueprintLibrary.AddLooseGameplayTags` (`self.GetAvatarActorFromActorInfo`) (`self.SwordThrewTAg`)))