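; Gameplay ability that teleports the main character to its sword instance and triggers retrieval of the sword.
; If the sword is valid, it moves the avatar to the sword's X/Y without sweeping, using the capsule half height as an absolute world Z.
; It then plays a 2D sound, activates the sword retrieval ability by tag and ends.
; With no valid sword, the ability never calls EndAbility.
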(event `self.K2_ActivateAbility`
  (bind _returnvalue (`self.GetAvatarActorFromActorInfo`))
  (bind _asbp_main_character (cast `/Game/Core/Character/BP_MainCharacter` _returnvalue :!pure true))
  (bind _swordinstance (`/Game/Core/Character/BP_MainCharacter.SwordInstance` _asbp_main_character)
    (:`then`
      (bind (_returnvalue_x _returnvalue_y) (`KismetMathLibrary.BreakVector` (`Actor.K2_GetActorLocation` _swordinstance)))
      (`Actor.K2_SetActorLocation` _returnvalue (`KismetMathLibrary.MakeVector` _returnvalue_x _returnvalue_y (`CapsuleComponent.CapsuleHalfHeight` (`Character.CapsuleComponent` _asbp_main_character))) false false)
      (`GameplayStatics.PlaySound2D` "/Game/Audio/Character/Teleport/SFX_TeleportUsed.SFX_TeleportUsed" 1.0 1.0 0.0 null null)
      (`AbilitySystemComponent.TryActivateAbilitiesByTag` (`AbilitySystemBlueprintLibrary.GetAbilitySystemComponent` _returnvalue) (`self.RetrieveSwordTag`) true)
      (`self.K2_EndAbility`))
    (:`else`)))