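; Gameplay ability that handles the player character's death and ends the game.
; On activation it stops the player controller's tick, disables controls and sets the Dead flag on the character's animation instance.
; It then plays the death montage and, when that completes, calls GameOver on the GM_Jam game mode as a player death.
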(event `self.K2_ActivateAbility`
  (bind _returnvalue (`GameplayStatics.GetPlayerController` 0))
  (`Actor.SetActorTickEnabled` _returnvalue false)
  (bind _ascharacter_controller (cast `CharacterController` _returnvalue))
  (`CharacterController.ToggleControls` _ascharacter_controller false)
  (`KismetSystemLibrary.PrintString` "DEATH")
  (bind _asabp_character_anim_instance (cast `/Game/Core/Character/Animation/ABP_CharacterAnimInstance` (`SkeletalMeshComponent.GetAnimInstance` (`Character.Mesh` (`GameplayStatics.GetPlayerCharacter` 0)))))
  (set `/Game/Core/Character/Animation/ABP_CharacterAnimInstance.Dead` true _asabp_character_anim_instance)
  (`AbilityTask_PlayMontageAndWait.CreatePlayMontageAndWaitProxy` "None" "/Game/AssetPack/CharacterPack/AnimationsSequence/AM_CharacterDeath.AM_CharacterDeath"
    (:`OnCompleted`
      (`/Game/Core/GameMode/GM_Jam.GameOver` (cast `/Game/Core/GameMode/GM_Jam` (`GameplayStatics.GetGameMode`) :!pure true) true false false))))