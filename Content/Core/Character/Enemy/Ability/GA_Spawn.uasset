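; Gameplay Ability that plays an enemy's spawn-from-ground entrance using a skeleton warrior montage.
; While the montage plays, it sets the AI blackboard's Stop flag, makes the capsule ignore pawns and unhides the enemy after a short delay.
; When the montage completes, blends out, is interrupted or cancelled, it restores AI and collision, registers the enemy through JamGameMode's InitializeEnemy and ends.
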(event `self.K2_ActivateAbility`
  (bind _asenemy (cast `Enemy` (`self.GetAvatarActorFromActorInfo`)))
  (bind _output_get (set `self.As Enemy` _asenemy))
  (`AbilityTask_PlayMontageAndWait.CreatePlayMontageAndWaitProxy` "None" "/Game/AssetPack/SkeletonsPack/Mesh/Character/AnimationSequence/Warrior/AM_Skeleton_Warrior_Anim_Spawn_Ground_Skeletons_Montage.AM_Skeleton_Warrior_Anim_Spawn_Ground_Skeletons_Montage"
    (:`then`
      (`BlackboardComponent.SetValueAsBool` (`AIController.Blackboard` (`AIBlueprintHelperLibrary.GetAIController` (`self.GetAvatarActorFromActorInfo`))) "Stop" true)
      (`PrimitiveComponent.SetCollisionResponseToChannel` (`Character.CapsuleComponent` (`self.As Enemy`)) "ECC_Pawn" "ECR_Ignore")
      (`AbilityTask_WaitDelay.WaitDelay` 0.5
        (:`OnFinish`
          (`Actor.SetActorHiddenInGame` _output_get false))))
    (:`OnCompleted`
      (`BlackboardComponent.SetValueAsBool` (`AIController.Blackboard` (`AIBlueprintHelperLibrary.GetAIController` (`self.GetAvatarActorFromActorInfo`))) "Stop" false :!label _label)
      (`PrimitiveComponent.SetCollisionResponseToChannel` (`Character.CapsuleComponent` (`self.As Enemy`)) "ECC_Pawn" "ECR_Block")
      (bind _asjam_game_mode (cast `JamGameMode` (`GameplayStatics.GetGameMode`)))
      (`JamGameMode.InitializeEnemy` _asjam_game_mode (`self.As Enemy`))
      (`self.K2_EndAbility`))
    (:`OnBlendOut`
      (goto _label))
    (:`OnInterrupted`
      (goto _label))
    (:`OnCancelled`
      (goto _label))))