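; Gameplay ability that puts an enemy into a knockback down-death state.
; On activation it adds Broken and DownDeath tags, sets the AI blackboard Stop flag and applies the GE_ReviveDelay effect.
; It makes the capsule ignore pawns and plays the skeleton warrior death montage, with no montage callbacks wired to end the ability.
; Ending removes only the Broken tag, leaving DownDeath, Stop and collision changes in place.
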(event `self.K2_ActivateAbility`
  (bind _returnvalue (`self.GetAvatarActorFromActorInfo`))
  (`AbilitySystemBlueprintLibrary.AddLooseGameplayTags` _returnvalue (`BlueprintGameplayTagLibrary.MakeLiteralGameplayTagContainer` (struct :`GameplayTags` (struct :`(TagName` "Status.Broken")))))
  (`AbilitySystemBlueprintLibrary.AddLooseGameplayTags` _returnvalue (`BlueprintGameplayTagLibrary.MakeLiteralGameplayTagContainer` (struct :`GameplayTags` (struct :`(TagName` "Status.DownDeath")))))
  (bind _output_get (set `self.Controller` (`AIBlueprintHelperLibrary.GetAIController` _returnvalue)))
  (`BlackboardComponent.SetValueAsBool` (`AIController.Blackboard` _output_get) "Stop" true)
  (`self.BP_ApplyGameplayEffectToOwner` "/Game/Core/Character/Enemy/Effect/GE_ReviveDelay.GE_ReviveDelay_C")
  (bind _ascharacter (cast `Character` (`self.GetAvatarActorFromActorInfo`))
    (:`then`
      (bind _output_get_2 (set `self.As Character` _ascharacter))
      (bind _capsulecomponent (`Character.CapsuleComponent` _output_get_2))
      (`PrimitiveComponent.SetCollisionResponseToChannel` _capsulecomponent "ECC_Pawn" "ECR_Ignore")
      (`PrimitiveComponent.SetCollisionObjectType` _capsulecomponent "ECC_Pawn")
      (`AbilityTask_PlayMontageAndWait.CreatePlayMontageAndWaitProxy` "None" "/Game/AssetPack/SkeletonsPack/Mesh/Character/AnimationSequence/Warrior/AM_Skeleton_Warior_Death.AM_Skeleton_Warior_Death"))
    (:`CastFailed`
      (`self.K2_EndAbility`))))

(event `self.K2_OnEndAbility`
  (params (bWasCancelled :type Boolean))
  (`AbilitySystemBlueprintLibrary.RemoveLooseGameplayTags` (`self.GetAvatarActorFromActorInfo`) (`BlueprintGameplayTagLibrary.MakeLiteralGameplayTagContainer` (struct :`GameplayTags` (struct :`(TagName` "Status.Broken"))))))