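; Enemy gameplay ability that puts an AI character into a knocked-down, broken state for the duration of a knockback effect.
; On activation it adds Status.Broken, sets the blackboard Stop flag, applies GE_DownKnockback, stops pawn collision blocking and disables actor tick.
; The down montage plays until the effect's removal jumps it to EndLoop.
; When it finishes, Stop, collision and the tag are restored if the controller is valid, but tick stays disabled.
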(event `self.K2_ActivateAbility`
  (bind _returnvalue (`self.GetAvatarActorFromActorInfo`))
  (bind _controller (`self.Controller`))
  (bind _capsulecomponent (`Character.CapsuleComponent` (`self.As Character`)))
  (`AbilitySystemBlueprintLibrary.AddLooseGameplayTags` _returnvalue (`BlueprintGameplayTagLibrary.MakeLiteralGameplayTagContainer` (struct :`GameplayTags` (struct :`(TagName` "Status.Broken")))))
  (bind _output_get (set `self.Controller` (`AIBlueprintHelperLibrary.GetAIController` _returnvalue)))
  (`BlackboardComponent.SetValueAsBool` (`AIController.Blackboard` _output_get) "Stop" true)
  (bind _returnvalue_2 (`self.BP_ApplyGameplayEffectToOwner` "/Game/Core/Character/Enemy/Effect/GE_DownKnockback.GE_DownKnockback_C"))
  (bind _ascharacter (cast `Character` (`self.GetAvatarActorFromActorInfo`))
    (:`then`
      (bind _output_get_2 (set `self.As Character` _ascharacter))
      (bind _capsulecomponent_2 (`Character.CapsuleComponent` _output_get_2))
      (`PrimitiveComponent.SetCollisionObjectType` _capsulecomponent_2 "ECC_Pawn")
      (`PrimitiveComponent.SetCollisionResponseToChannel` _capsulecomponent_2 "ECC_Pawn" "ECR_Ignore")
      (`Actor.SetActorTickEnabled` _output_get_2 false)
      (`AbilityTask_PlayMontageAndWait.CreatePlayMontageAndWaitProxy` "None" "/Game/AssetPack/SkeletonsPack/Mesh/Character/AnimationSequence/Warrior/AM_Skeleton_Warior_Down.AM_Skeleton_Warior_Down"
        (:`then`
          (`AbilityTask_WaitGameplayEffectRemoved.WaitForGameplayEffectRemoved` _returnvalue_2
            (:`OnRemoved`
              (`self.MontageJumpToSection` "EndLoop"))))
        (:`OnCompleted`
          (`/Engine/EditorBlueprintResources/StandardMacros.IsValid` _controller :!label _label
            (:`Is Valid`
              (`BlackboardComponent.SetValueAsBool` (`AIController.Blackboard` _controller) "Stop" false)
              (`PrimitiveComponent.SetCollisionResponseToChannel` _capsulecomponent "ECC_Pawn" "ECR_Block")
              (`PrimitiveComponent.SetCollisionObjectType` _capsulecomponent "ECC_GameTraceChannel3")
              (`AbilitySystemBlueprintLibrary.RemoveLooseGameplayTags` (`self.GetAvatarActorFromActorInfo`) (`BlueprintGameplayTagLibrary.MakeLiteralGameplayTagContainer` (struct :`GameplayTags` (struct :`(TagName` "Status.Broken")))))
              (`self.K2_EndAbility`))
            (:`Is Not Valid`
              (`self.K2_EndAbility`))))
        (:`OnBlendOut`
          (goto _label))
        (:`OnInterrupted`
          (goto _label))
        (:`OnCancelled`
          (goto _label))))
    (:`CastFailed`
      (`self.K2_EndAbility`))))