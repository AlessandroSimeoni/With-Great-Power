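; Gameplay ability that revives a downed enemy with the AM_WarriorResurrect montage.
; On activation it starts the montage and removes the Status.DownDeath loose tag from the avatar.
; However the montage exits, it clears the AI blackboard Stop flag, restores capsule collision and actor tick, and calls EnemyRevive before ending.
; Debug prints remain in the flow.
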(event `self.K2_ActivateAbility`
  (`AbilityTask_PlayMontageAndWait.CreatePlayMontageAndWaitProxy` "None" "/Game/AssetPack/SkeletonsPack/Mesh/Character/AnimationSequence/Warrior/AM_WarriorResurrect.AM_WarriorResurrect"
    (:`then`
      (`AbilitySystemBlueprintLibrary.RemoveLooseGameplayTags` (`self.GetAvatarActorFromActorInfo`) (`BlueprintGameplayTagLibrary.MakeLiteralGameplayTagContainer` (struct :`GameplayTags` (struct :`(TagName` "Status.DownDeath")))))
      (`KismetSystemLibrary.PrintString` "Remove Tag"))
    (:`OnCompleted`
      (bind _asenemy (cast `Enemy` (`self.GetAvatarActorFromActorInfo`) :!label _label)
        (:`then`
          (`BlackboardComponent.SetValueAsBool` (`AIController.Blackboard` (`AIBlueprintHelperLibrary.GetAIController` (`self.GetAvatarActorFromActorInfo`))) "Stop" false)
          (bind _capsulecomponent (`Character.CapsuleComponent` _asenemy))
          (`PrimitiveComponent.SetCollisionResponseToChannel` _capsulecomponent "ECC_Pawn" "ECR_Block")
          (`PrimitiveComponent.SetCollisionObjectType` _capsulecomponent "ECC_GameTraceChannel3")
          (`Actor.SetActorTickEnabled` _asenemy true)
          (`Enemy.EnemyRevive` _asenemy)
          (`self.K2_EndAbility`)
          (`KismetSystemLibrary.PrintString` "Hello"))
        (:`CastFailed`
          (`self.K2_EndAbility`))))
    (:`OnBlendOut`
      (goto _label))
    (:`OnInterrupted`
      (goto _label))
    (:`OnCancelled`
      (goto _label))))