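; Gameplay ability that makes an Enemy focus its AI controller on the target supplied by the triggering gameplay event.
; On activation it switches the enemy's movement mode, enables the controller's tick and sets focus on that target.
; It stays active until a cancel input ends it, then OnEndAbility restores the movement mode, clears focus and disables the controller's tick.
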(event `self.K2_ActivateAbilityFromEvent`
  (params (EventData :type "GameplayEventData Structure (by ref)"))
  (bind _returnvalue (`self.GetAvatarActorFromActorInfo`))
  (bind _asenemy (cast `Enemy` _returnvalue))
  (`Enemy.SwitchMovementMode` _asenemy true)
  (bind _asaicontroller (cast `AIController` (`Pawn.GetController` (`Actor.Instigator` _returnvalue))))
  (`Actor.SetActorTickEnabled` _asaicontroller true)
  (`AIController.K2_SetFocus` _asaicontroller EventData_Target)
  (`AbilityTask_WaitCancel.WaitCancel`
    (:`OnCancel`
      (`self.K2_EndAbility`))))

(event `self.K2_OnEndAbility`
  (params (bWasCancelled :type Boolean))
  (bind _asenemy (cast `Enemy` (`self.GetAvatarActorFromActorInfo`)))
  (`Enemy.SwitchMovementMode` _asenemy false)
  (bind _asaicontroller (cast `AIController` (`Pawn.GetController` _asenemy)))
  (`AIController.K2_ClearFocus` _asaicontroller)
  (`Actor.SetActorTickEnabled` (`AIBlueprintHelperLibrary.GetAIController` (`self.GetAvatarActorFromActorInfo`)) false))