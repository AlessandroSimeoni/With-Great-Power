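; GA_Shoot is an event-activated Gameplay Ability that makes the enemy BP_Archer fire an arrow at the event's target.
; It plays a ranged shoot montage and waits for the Event.Shoot gameplay event to time the release.
; On that event, the archer's MuzzlesController launches a targeted arrow projectile, with damage read from a gameplay attribute, and prints a debug string.
; The ability ends when the montage completes, blends out, is interrupted or is cancelled.
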(event `self.K2_ActivateAbilityFromEvent`
  (params (EventData :type "GameplayEventData Structure (by ref)"))
  (set `self.Target` EventData_Target)
  (`AbilityTask_PlayMontageAndWait.CreatePlayMontageAndWaitProxy` "None" "/Game/AssetPack/SkeletonsPack/Mesh/Character/AnimationSequence/Rogue/AM_Skeleton_Rogue_Anim_1H_Ranged_Shoot_Montage.AM_Skeleton_Rogue_Anim_1H_Ranged_Shoot_Montage"
    (:`then`
      (`AbilityTask_WaitGameplayEvent.WaitGameplayEvent` (struct :`TagName` "Event.Shoot") null
        (:`EventReceived`
          (bind _asbp_archer (cast `/Game/Core/Character/Enemy/Archer/BP_Archer` (`self.GetAvatarActorFromActorInfo`)))
          (`MuzzlesController.ShootWithMuzzle` (`/Game/Core/Character/Enemy/Archer/BP_Archer.MuzzlesController` _asbp_archer) 0 "/Game/Core/Character/Enemy/Projectile/BP_StraightTargetProjectile_Arrow.BP_StraightTargetProjectile_Arrow_C" 800.0 (`self.Target`) (`.ReturnValue` (`AbilitySystemComponent.GetGameplayAttributeValue` (`self.GetAbilitySystemComponentFromActorInfo`) (struct :`AttributeName` "Attack" :`Attribute` "/Script/KenneyJam.EnemyAttributeSet:Attack" :`AttributeOwner` "/Script/CoreUObject.Class'/Script/KenneyJam.EnemyAttributeSet'"))) 0.0 1.0)
          (`KismetSystemLibrary.PrintString` "Shoot"))))
    (:`OnCompleted`
      (`self.K2_EndAbility` :!label _label))
    (:`OnBlendOut`
      (goto _label))
    (:`OnInterrupted`
      (goto _label))
    (:`OnCancelled`
      (goto _label))))