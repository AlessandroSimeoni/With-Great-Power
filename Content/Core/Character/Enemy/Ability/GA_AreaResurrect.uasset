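; Enemy gameplay ability that periodically attempts to revive enemies around its owner.
; On activation it starts a looping timer that, each interval, plays the skeleton mage raise montage and runs Resurrect as the montage starts, without waiting for completion.
; Resurrect sphere-overlaps BP_BaseEnemy pawns within Area and tries to activate GA_Revive on each one's ability system component, with debug sphere and print output.
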(event `self.K2_ActivateAbility`
  (`KismetSystemLibrary.K2_SetTimerDelegate` (delegate `CustomEvent`) (`self.Interval`) true))

(event `CustomEvent`
  (`AbilityTask_PlayMontageAndWait.CreatePlayMontageAndWaitProxy` "None" "/Game/AssetPack/SkeletonsPack/Mesh/Character/AnimationSequence/Mage/Skeleton_Mage_Anim_Spellcast_Raise_Montage.Skeleton_Mage_Anim_Spellcast_Raise_Montage"
    (:`then`
      (`self.Resurrect`)
      (`KismetSystemLibrary.PrintString` "Resurrect"))))

(fn `Resurrect`
  (bind _area (`self.Area`))
  (bind _returnvalue (`Actor.K2_GetActorLocation` (`self.GetAvatarActorFromActorInfo`)))
  (`KismetSystemLibrary.DrawDebugSphere` _returnvalue _area 12 (struct :`G` 0.151564 :`B` 1.0 :`A` 1.0) 1.0)
  (bind _outactors (`KismetSystemLibrary.SphereOverlapActors` _returnvalue _area (`|MakeArray` "ObjectTypeQuery3" :!type "EObjectTypeQuery Enum") "/Game/Core/Character/Enemy/BP_BaseEnemy.BP_BaseEnemy_C"))
  (for _array_element _outactors
    (`AbilitySystemComponent.TryActivateAbilityByClass` (`AbilitySystemBlueprintLibrary.GetAbilitySystemComponent` _array_element) "/Game/Core/Character/Enemy/Ability/GA_Revive.GA_Revive_C" true)))