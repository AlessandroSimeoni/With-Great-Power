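; Gameplay ability for the Warrior enemy's leaping melee chop attack, activated by a gameplay event.
; It instantly rotates the avatar to face the event's instigator, then applies a short forward root-motion jump force.
; The skeleton warrior jump-chop montage starts alongside the jump, and the ability ends when it completes, blends out, or is interrupted or cancelled.
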(event `self.K2_ActivateAbilityFromEvent`
  (params (EventData :type "GameplayEventData Structure (by ref)"))
  (bind _returnvalue (`self.GetAvatarActorFromActorInfo`))
  (bind (_returnvalue_roll _returnvalue_pitch _returnvalue_yaw) (`KismetMathLibrary.BreakRotator` (`Actor.K2_GetActorRotation` _returnvalue)))
  (bind (_returnvalue_roll_2 _returnvalue_pitch_2 _returnvalue_yaw_2) (`KismetMathLibrary.BreakRotator` (`KismetMathLibrary.FindLookAtRotation` (`Actor.K2_GetActorLocation` _returnvalue) (`Actor.K2_GetActorLocation` EventData_Instigator))))
  (`TaskRotateCharacter.RotateCharacter` "None" (- _returnvalue_yaw_2 _returnvalue_yaw) 0.0 null
    (:`OnRotationCompleted`
      (`AbilityTask_ApplyRootMotionJumpForce.ApplyRootMotionJumpForce` "None" (`KismetMathLibrary.Conv_VectorToRotator` (`Actor.GetActorForwardVector` (`self.GetAvatarActorFromActorInfo`))) 500.0 200.0 0.3 0.0 false "MaintainLastRootMotionVelocity"
        (:`then`
          (`AbilityTask_PlayMontageAndWait.CreatePlayMontageAndWaitProxy` "None" "/Game/AssetPack/SkeletonsPack/Mesh/Character/AnimationSequence/Warrior/Skeleton_Warrior_Anim_1H_Melee_Attack_Jump_Chop_Montage.Skeleton_Warrior_Anim_1H_Melee_Attack_Jump_Chop_Montage"
            (:`OnCompleted`
              _)
            (:`OnBlendOut`
              _)
            (:`OnInterrupted`
              _)
            (:`OnCancelled`
              _))
          (`self.K2_EndAbility`))))))

(event `self.K2_ActivateAbility`)