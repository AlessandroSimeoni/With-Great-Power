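; Player character that throws and retrieves a sword actor, BP_Sword.
; On BeginPlay it finds the sword already in the level and calls SetWeaponOwner on it.
; Left mouse throws it along the actor's forward vector with a viewport mouse target point, packing the UseMouse flag into Z; right mouse retrieves it.
; Holding IA_Throw past SustainThreshold sets the sword's CanSustain flag, cleared on completion.
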(event `self.ReceiveBeginPlay`
  (`parent.ReceiveBeginPlay`)
  (bind _returnvalue (`GameplayStatics.GetActorOfClass` "/Game/Core/Actor/Weapons/BP_Sword.BP_Sword_C"))
  (bind _output_get (set `self.WeaponSword` _returnvalue))
  (`WeaponSword.SetWeaponOwner` _output_get null))

(event `self.ReceiveActorBeginOverlap`
  (params (OtherActor :type "Actor Object Reference")))

(event `self.ReceiveTick`
  (params (DeltaSeconds :type "Float (single-precision)")))

(event `Key|LeftMouseButton`
  (params (Key :type "Key Structure"))
  (:`Pressed`
    (bind _returnvalue (`WidgetLayoutLibrary.GetMousePositionOnViewport`))
    (`WeaponSword.ThrowWeapon` (`self.WeaponSword`) (`self.Velocity`) (`self.Force`) (`self.Damage`) (`self.GetActorForwardVector`) (`KismetMathLibrary.Conv_Vector2DToVector` _returnvalue (`KismetMathLibrary.Conv_BoolToDouble` (`self.UseMouse`))))))

(event `Key|RightMouseButton`
  (params (Key :type "Key Structure"))
  (:`Pressed`
    (`WeaponSword.RetrieveWeapon` (`self.WeaponSword`))))

(event `EnhancedInput|/Game/Core/Input/IA_Throw`
  (params (ActionValue :type Boolean) (ElapsedSeconds :type "Float (double-precision)") (TriggeredSeconds :type "Float (double-precision)") (InputAction :type "InputAction Object Reference" :default "/Game/Core/Input/IA_Throw.IA_Throw"))
  (:`Ongoing`
    (set `WeaponSword.bCanSustain` (> ElapsedSeconds (`self.SustainThreshold`)) (`self.WeaponSword`)))
  (:`Completed`
    (set `WeaponSword.bCanSustain` false (`self.WeaponSword`))))

(fn `UserConstructionScript`
  (`parent.UserConstructionScript`))