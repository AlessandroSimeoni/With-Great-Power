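; Main character Blueprint for a charged sword throw and recall, built on the Gameplay Ability System.
; Tick fills a progress-bar widget at the attribute set's charge speed, activating GA_ThrowWeapon when full, while chained timelines animate camera FOV and arm length.
; ThrowSword hides the socketed weapon and launches a spawned BP_Sword, with speed and force scaled by charge.
; Completed retrieval destroys it, reshows the weapon and sends a gameplay event.
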(event `self.ReceiveBeginPlay`
  (`self.AttachWeaponToSocket`)
  (bind _asw_attack_progress (cast `/Game/UI/W_AttackProgress` (`WidgetComponent.GetWidget` (`self.AttackProgress`))))
  (set `self.AttackProgressBarWidget` _asw_attack_progress)
  (bind _returnvalue (`AbilitySystemComponent.GetAttributeSet` (`self.AbilitySystemComponent`) "/Script/KenneyJam.PlayerAttributeSet"))
  (bind _asplayer_attribute_set (cast `PlayerAttributeSet` _returnvalue))
  (set `self.ChargeSpeed` (`.BaseValue` (break `GameplayAttributeData` (`PlayerAttributeSet.MaxChargeSpeed` _asplayer_attribute_set)))))

(event `self.ReceiveTick`
  (params (DeltaSeconds :type "Float (single-precision)"))
  (bind _attackprogressbarwidget (`self.AttackProgressBarWidget`))
  (bind _percent (`ProgressBar.Percent` (`/Game/UI/W_AttackProgress.ProgressBar_0` _attackprogressbarwidget)))
  (if (`self.IncrementAttackProgress`)
    (`/Game/UI/W_AttackProgress.UpdateProgressBar` _attackprogressbarwidget (`KismetMathLibrary.FClamp` (+ (* DeltaSeconds (`self.ChargeSpeed`)) _percent)))
    (if (== _percent 1.0)
      (`AbilitySystemComponent.TryActivateAbilityByClass` (`self.AbilitySystemComponent`) "/Game/Core/Character/Abilities/GA_ThrowWeapon.GA_ThrowWeapon_C" true))))

(event `RetrieveSwordCompleted_Event`
  (`self.K2_DestroyActor` (`self.SwordInstance`))
  (`SceneComponent.SetVisibility` (`self.Weapon`) true false)
  (`AbilitySystemBlueprintLibrary.SendGameplayEventToActor` self (struct :`TagName` "Event.SwordRetrieved")))

(event `StartCameraMovementWhenCharging`
  (bind _camera (`self.Camera`))
  ;[1 1 1] Camera nightmare
  (set `self.InitialFOV` (`CameraComponent.FieldOfView` _camera))
  (set `self.InitialArmLength` (`SpringArmComponent.TargetArmLength` (`self.SpringArm`)))
  (bind (_direction _test_fov) (`Timeline|Timeline_1` :!via `PlayFromStart`)
    (:`Update`
      (bind _returnvalue (`KismetMathLibrary.Lerp` (`self.InitialFOV`) 110.0 _test_fov))
      (`CameraComponent.SetFieldOfView` _camera _returnvalue)
      (set `self.LastFOV` _returnvalue)
      (bind (_direction_2 _test_fov_2) (`Timeline|Timeline_2` :!via `PlayFromStart`)
        (:`Update`
          (bind _output_get (set `SpringArmComponent.TargetArmLength` (`KismetMathLibrary.Lerp` (`self.InitialArmLength`) 3500.0 _test_fov_2) (`self.SpringArm`)))
          (set `self.LastArmLength` _output_get))
        (:`Finished`
          (bind (_direction_3 _armlenght) (`Timeline|Timeline_4` :!via `PlayFromStart` :!label _label)
            (:`Update`
              (set `SpringArmComponent.TargetArmLength` (`KismetMathLibrary.Lerp` (`self.LastArmLength`) (`self.InitialArmLength`) _armlenght) (`self.SpringArm`)))))))
    (:`Finished`
      (`self.Reset Fov`))))

(event `Reset Fov`
  ;[1 1 1] Camera nightmare
  (`TimelineComponent.SetPlayRate` (`self.Timeline_3`) 5.0)
  (bind (_direction _test_fov) (`Timeline|Timeline_3` :!via `PlayFromStart`)
    (:`Update`
      (`CameraComponent.SetFieldOfView` (`self.Camera`) (`KismetMathLibrary.Lerp` (`self.LastFOV`) (`self.InitialFOV`) _test_fov)))))

(event `StopCameraMovement`
  (bind _timeline_1 (`self.Timeline_1`))
  (bind _timeline_2 (`self.Timeline_2`))
  ;[1 1 1] Camera nightmare
  (if (`TimelineComponent.IsPlaying` _timeline_1)
    (`TimelineComponent.Stop` _timeline_1)
    (`self.Reset Fov`)
    (if (`TimelineComponent.IsPlaying` _timeline_2)
      (`TimelineComponent.Stop` _timeline_2)
      (goto _label :!via `PlayFromStart`))))

(fn `AttachWeaponToSocket`
  (`SceneComponent.K2_AttachToComponent` (`self.Weapon`) (`self.Mesh`) "WeaponSocket" "SnapToTarget" "SnapToTarget" "KeepWorld" true))

(fn `BeginThrowAction`
  (`/Game/UI/W_AttackProgress.ShowProgressBar` (`self.AttackProgressBarWidget`))
  (set `self.IncrementAttackProgress` true)
  (`self.StartCameraMovementWhenCharging`))

(fn `RetrieveSword`
  (bind _swordinstance (`self.SwordInstance`)
    (:`then`
      (add `WeaponSword.OnRetrieveCompleted` _swordinstance (`|CreateDelegate` :!event `RetrieveSwordCompleted_Event`))
      ;[1 0 0.01364] MANCA EVENTO DI RETRIEVE SPADA PER CAPIRE QUANDO MI ARRIVA ADDOSSO, POI DISTRUGGO SPADA E SEND EVENT CON TAG Event.SwordRetrieved
      (`WeaponSword.RetrieveWeapon` _swordinstance))
    (:`else`)))

(fn `StopChargeBar`
  (`/Game/UI/W_AttackProgress.HideProgressBar` (`self.AttackProgressBarWidget`))
  (set `self.IncrementAttackProgress` false))

(fn `ThrowSword`
  (bind _arrow1 (`self.Arrow1`))
  (bind _percent (`ProgressBar.Percent` (`/Game/UI/W_AttackProgress.ProgressBar_0` (`self.AttackProgressBarWidget`))))
  (`SceneComponent.SetVisibility` (`self.Weapon`) false false)
  (bind _returnvalue (`|SpawnActorFromClass` "/Game/Core/Actor/Weapons/BP_Sword.BP_Sword_C" (`KismetMathLibrary.MakeTransform` (`SceneComponent.K2_GetComponentLocation` _arrow1) (`SceneComponent.K2_GetComponentRotation` _arrow1)) "AlwaysSpawn" "MultiplyWithRoot" null null))
  (bind _output_get (set `self.SwordInstance` _returnvalue))
  (bind _returnvalue_2 (`AbilitySystemComponent.GetAttributeSet` (`self.AbilitySystemComponent`) "/Script/KenneyJam.PlayerAttributeSet"))
  (bind _asplayer_attribute_set (cast `PlayerAttributeSet` _returnvalue_2))
  (bind (_throwingweaponspeed_basevalue _throwingweaponspeed_currentvalue) (break `GameplayAttributeData` (`PlayerAttributeSet.ThrowingWeaponSpeed` _asplayer_attribute_set)))
  (bind (_throwingweaponforce_basevalue _throwingweaponforce_currentvalue) (break `GameplayAttributeData` (`PlayerAttributeSet.ThrowingWeaponForce` _asplayer_attribute_set)))
  (`WeaponSword.ThrowWeapon` _output_get (* _percent _throwingweaponspeed_currentvalue) (* _percent _throwingweaponforce_currentvalue) 1.0 (`self.GetActorForwardVector`) (`KismetMathLibrary.Vector_Zero`))
  (`WeaponSword.ThrowWeapon` _output_get (* _percent _throwingweaponspeed_currentvalue) (* _percent _throwingweaponforce_currentvalue) 1.0 (`self.GetActorForwardVector`) (`KismetMathLibrary.Vector_Zero`))
  (`self.StopCameraMovement`))

(fn `UserConstructionScript`)