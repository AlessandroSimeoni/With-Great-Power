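; Game mode for a jam level that runs the HUD, music and win/lose flow around enemy count and city destruction.
; Event handlers feed the HUD counter and slider: zero enemies wins, while a low destruction percentage loses through GameOver, which also handles player death and out-of-bounds.
; Building destruction randomly triggers non-overlapping voice reactions that change at the halfway threshold, where a one-time event also swaps the soundtrack.
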(event `self.OnEnemyDied`
  (params (Enemy :type "Actor Object Reference") (TotalEnemyNumber :type "Float (single-precision)"))
  (bind _returnvalue (`GameplayStatics.GetPlayerController` 0))
  (`/Game/UI/WB_EnemyCounter.UpdateValue` (`/Game/UI/W_HUD.WB_EnemyCounter` (`self.HUD`)) (`KismetMathLibrary.FTrunc` TotalEnemyNumber) false)
  (if (and (<= TotalEnemyNumber 0.0) (not (`self.IsGameOver`)))
    (`CharacterController.ToggleControls` (cast `CharacterController` _returnvalue :!pure true) false)
    (`self.SetActorTickEnabled` _returnvalue false)
    (`self.GameOver` false false true)))

(event `self.ReceiveBeginPlay`
  (bind _returnvalue (`|CreateWidget` "/Game/UI/W_HUD.W_HUD_C"))
  (bind _output_get (set `self.HUD` _returnvalue))
  (`UserWidget.AddToViewport` _output_get 0)
  (bind _asbp_design_character (cast `/Game/Core/Character/BP_DesignCharacter` (`GameplayStatics.GetPlayerCharacter` 0)))
  (set `self.As BP Main Character` _asbp_design_character)
  (bind _returnvalue_2 (`GameplayStatics.SpawnSound2D` "/Game/Audio/SoundTrack/BGM_Level.BGM_Level" 1.0 1.0 0.0 null))
  (set `self.Soundtrack` _returnvalue_2))

(event `self.OnInitialization`
  (params (TotalEnemyNumber :type "Float (single-precision)") (TotalDestructionNumber :type "Float (single-precision)"))
  (bind _hud (`self.HUD`))
  (`/Game/UI/WB_EnemyCounter.SetValue` (`/Game/UI/W_HUD.WB_EnemyCounter` _hud) (`KismetMathLibrary.FTrunc` TotalEnemyNumber) false)
  (`/Game/UI/WB_SliderDestruction.SetValue` (`/Game/UI/W_HUD.WB_SliderDestruction` _hud) TotalDestructionNumber TotalDestructionNumber false))

(event `self.OnEnemyRevived`
  (params (Enemy :type "Actor Object Reference") (TotalEnemyNumber :type "Float (single-precision)"))
  (`/Game/UI/WB_EnemyCounter.UpdateValue` (`/Game/UI/W_HUD.WB_EnemyCounter` (`self.HUD`)) (`KismetMathLibrary.FTrunc` TotalEnemyNumber) false))

(event `self.OnBuildingDestroyed`
  (params (Building :type "Actor Object Reference") (TotalDestructionNumber :type "Float (single-precision)"))
  (bind _returnvalue (`GameplayStatics.GetPlayerController` 0))
  (bind _wb_sliderdestruction (`/Game/UI/W_HUD.WB_SliderDestruction` (`self.HUD`)))
  (`/Game/UI/WB_SliderDestruction.UpdateValue` _wb_sliderdestruction TotalDestructionNumber false)
  (bind _returnvalue_2 (`/Game/UI/WB_SliderDestruction.CalculateDestructionPercent` _wb_sliderdestruction))
  (`self.ReactionSound` _returnvalue_2)
  (if (and (<= _returnvalue_2 0.5) (not (`self.FirstEventDone`)))
    (set `self.FirstEventDone` true)
    (`self.FirstEvent`)
    (elif (and (<= _returnvalue_2 0.15) (not (`self.IsGameOver`)))
      (`CharacterController.ToggleControls` (cast `CharacterController` _returnvalue :!pure true) false)
      (`self.SetActorTickEnabled` _returnvalue false)
      (`self.GameOver` false true))))

(event `ReactionSound`
  (params (Percent :type "Float (double-precision)"))
  (bind _sfxreact (`self.SFXReact`))
  (if (> (`KismetMathLibrary.RandomIntegerInRange` 0 100) 80)
    (if (`KismetSystemLibrary.IsValid` _sfxreact)
      (if (not (`AudioComponent.IsPlaying` _sfxreact))
        (if (> Percent 0.5) :!label _label
          (bind _returnvalue (`GameplayStatics.SpawnSound2D` "/Game/Audio/VoiceOver/OhNo/SFX_Voice_OhNo_1_Cue.SFX_Voice_OhNo_1_Cue" 1.0 1.0 0.0 null))
          (set `self.SFXReact` _returnvalue)
          (else
            (bind _returnvalue_2 (`GameplayStatics.SpawnSound2D` (select `int` (`KismetMathLibrary.RandomIntegerInRange` 0 2) :`0` "/Game/Audio/VoiceOver/Laugh/SFX_Voice_BlackLaugh_Cue.SFX_Voice_BlackLaugh_Cue" :`1` "/Game/Audio/VoiceOver/Destroy/SFX_Voice_Destroy.SFX_Voice_Destroy" :`2` "/Game/Audio/VoiceOver/Power/SFX_Voice_Power_Cue.SFX_Voice_Power_Cue" :!type "SoundBase Object Reference") 1.0 1.0 0.0 null))
            (set `self.SFXReact` _returnvalue_2))))
      (else
        (goto _label)))))

(event `FirstEvent`
  (bind _soundtrack (`self.Soundtrack`))
  ;[1 1 1] TODO
  (if (`KismetSystemLibrary.IsValid` _soundtrack)
    (`AudioComponent.Stop` _soundtrack)
    (`GameplayStatics.SpawnSound2D` "/Game/Audio/VoiceOver/Laugh/SFX_Voice_BlackLaugh_2.SFX_Voice_BlackLaugh_2" 1.0 1.0 0.0 null))
  (bind _returnvalue (`GameplayStatics.SpawnSound2D` "/Game/Audio/SoundTrack/BGM_BlackKnight.BGM_BlackKnight" 1.0 1.0 0.0 null))
  (set `self.Soundtrack` _returnvalue))

(fn `GameOver`
  (params (PlayerDead :type Boolean) (CityDestroyed :type Boolean) (AllEnemiesDied :type Boolean) (OutOfBounds :type Boolean))
  (`Widget.RemoveFromParent` (`self.HUD`))
  (set `self.IsGameOver` true)
  (if (or PlayerDead CityDestroyed OutOfBounds)
    (bind _returnvalue (`|CreateWidget` "/Game/UI/WB_Lose.WB_Lose_C"))
    (`/Game/UI/WB_Lose.LoseCondition` _returnvalue OutOfBounds PlayerDead CityDestroyed)
    (`UserWidget.AddToViewport` _returnvalue 0)
    (elif AllEnemiesDied
      (bind _returnvalue_2 (`|CreateWidget` "/Game/UI/WB_Win.WB_Win_C"))
      (`UserWidget.AddToViewport` _returnvalue_2 0))))

(fn `UserConstructionScript`)